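; BP_Enemy is an enemy actor that the player can shoot for score or be hit by on contact.
; TriggerZone overlap with a BP_Projectile increments the score on the projectile's player reference and destroys both actors, while overlap with BP_Player calls ProcessHit and destroys the enemy.
; A second volume, PassZone, destroys the enemy when the player stops overlapping it, without changing the score.
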(event `self.TriggerZone.OnComponentBeginOverlap`
  (params (OverlappedComponent :type "PrimitiveComponent Object Reference") (OtherActor :type "Actor Object Reference") (OtherComp :type "PrimitiveComponent Object Reference") (OtherBodyIndex :type Integer) (bFromSweep :type Boolean) (SweepResult :type "HitResult Structure (by ref)"))
  (bind _asbp_projectile (cast `/Game/InfiniteMatrix/Blueprints/BP_Projectile` OtherActor)
    (:`then`
      (`/Engine/EditorBlueprintResources/StandardMacros.IncrementInt` (`/Game/InfiniteMatrix/Blueprints/BP_Player.Score` (`/Game/InfiniteMatrix/Blueprints/BP_Projectile.Player REF` _asbp_projectile))
        (:`  `
          (`self.K2_DestroyActor` _asbp_projectile)
          (`self.K2_DestroyActor`))))
    (:`CastFailed`
      (bind _asbp_player (cast `/Game/InfiniteMatrix/Blueprints/BP_Player` OtherActor))
      (`/Game/InfiniteMatrix/Blueprints/BP_Player.ProcessHit` _asbp_player)
      (`self.K2_DestroyActor`))))

(event `self.PassZone.OnComponentEndOverlap`
  (params (OverlappedComponent :type "PrimitiveComponent Object Reference") (OtherActor :type "Actor Object Reference") (OtherComp :type "PrimitiveComponent Object Reference") (OtherBodyIndex :type Integer))
  (cast `/Game/InfiniteMatrix/Blueprints/BP_Player` OtherActor)
  (`self.K2_DestroyActor`))

(fn `UserConstructionScript`)